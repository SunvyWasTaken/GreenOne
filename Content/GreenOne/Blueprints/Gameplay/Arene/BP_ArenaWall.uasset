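; BP_ArenaWall is an arena wall that becomes solid and visible when its arena is activated.
; Its mesh collision is disabled on BeginPlay, then the ArenaActive event sets the active flag, enables query and physics collision, and unhides the mesh with its children.
; The construction script writes ArenaId to a text render, labeling which arena the wall is assigned to.
; The file contains no logic to deactivate the wall again.
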(event `self.ReceiveBeginPlay`
  (`PrimitiveComponent.SetCollisionEnabled` (`self.StaticMesh`) "NoCollision"))

(event `ArenaActive`
  (bind _staticmesh (`self.StaticMesh`))
  (set `self.IsArenaActive` true)
  (`PrimitiveComponent.SetCollisionEnabled` _staticmesh "QueryAndPhysics")
  (`SceneComponent.SetHiddenInGame` _staticmesh false true))

(fn `UserConstructionScript`
  (`TextRenderComponent.K2_SetText` (`self.TextRender`) (`KismetTextLibrary.Conv_IntToText` (`self.ArenaId`))))