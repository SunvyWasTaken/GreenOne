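; A self-destroying trigger actor that shows two pop-up widgets in sequence when BP_Player overlaps its Box component.
; The first widget stays in the viewport for a set delay, then is removed and replaced by the second for its own delay.
; Widget classes and display times come from variables, and the actor destroys itself after removing the second widget.
; No guard blocks repeat overlaps while the sequence runs.
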(event `self.ReceiveBeginPlay`)

(event `self.Box.OnComponentBeginOverlap`
  (params (OverlappedComponent :type "PrimitiveComponent Object Reference") (OtherActor :type "Actor Object Reference") (OtherComp :type "PrimitiveComponent Object Reference") (OtherBodyIndex :type Integer) (bFromSweep :type Boolean) (SweepResult :type "HitResult Structure (by ref)"))
  (cast `/Game/GreenOne/Blueprints/BP_Player` OtherActor)
  (bind _returnvalue (`|CreateWidget` (`self.WBP_Class`)))
  (`UserWidget.AddToViewport` _returnvalue 0)
  (`KismetSystemLibrary.Delay` (`self.DestroyWBPTime`))
  (`Widget.RemoveFromParent` _returnvalue)
  (bind _returnvalue_2 (`|CreateWidget` (`self.WBP_Class_deux`)))
  (`UserWidget.AddToViewport` _returnvalue_2 0)
  (`KismetSystemLibrary.Delay` (`self.DestroyWBPTimedeux`))
  (`Widget.RemoveFromParent` _returnvalue_2)
  (`self.K2_DestroyActor`))

(fn `UserConstructionScript`)