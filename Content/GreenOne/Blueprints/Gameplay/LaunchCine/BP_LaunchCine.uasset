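; BP_LaunchCine is a trigger actor that plays a cinematic Level Sequence the first time the player character overlaps its Box.
; A DoOnce gate blocks repeat triggers, then a sequence player is created from the LevelSequence and settings variables and started.
; IsPlaying is set true at the start and cleared by a Delay matching the sequence's duration, rather than by a finished event.
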(event `self.Box.OnComponentBeginOverlap`
  (params (OverlappedComponent :type "PrimitiveComponent Object Reference") (OtherActor :type "Actor Object Reference") (OtherComp :type "PrimitiveComponent Object Reference") (OtherBodyIndex :type Integer) (bFromSweep :type Boolean) (SweepResult :type "HitResult Structure (by ref)"))
  (if (== OtherActor (`GameplayStatics.GetPlayerCharacter` 0))
    (`/Engine/EditorBlueprintResources/StandardMacros.DoOnce` false
      (:`Completed`
        (set `self.IsPlaying` true)
        (bind (_outactor _returnvalue) (`LevelSequencePlayer.CreateLevelSequencePlayer` (`self.LevelSequence`) (`self.LevelSequenceSettings`)))
        (`MovieSceneSequencePlayer.Play` (`LevelSequenceActor.SequencePlayer` _outactor))
        (`KismetSystemLibrary.Delay` (`TimeManagementBlueprintLibrary.Conv_QualifiedFrameTimeToSeconds` (`MovieSceneSequencePlayer.GetDuration` _returnvalue)))
        (set `self.IsPlaying` false)))))

(fn `UserConstructionScript`)