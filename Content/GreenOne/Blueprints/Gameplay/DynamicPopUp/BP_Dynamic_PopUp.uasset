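; A trigger actor that shows a timed on-screen pop-up message when the player character overlaps its box.
; After a configurable delay, a DoOnce lets the pop-up fire a single time, creating a WBP_DynamicPopUp widget and adding it to the viewport.
; Text and background color pass to the widget through the BPI_DynamicPopUp interface, and the widget is removed after a set on-screen time.
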(event `self.Box.OnComponentBeginOverlap`
  (params (OverlappedComponent :type "PrimitiveComponent Object Reference") (OtherActor :type "Actor Object Reference") (OtherComp :type "PrimitiveComponent Object Reference") (OtherBodyIndex :type Integer) (bFromSweep :type Boolean) (SweepResult :type "HitResult Structure (by ref)"))
  (if (== OtherActor (`GameplayStatics.GetPlayerCharacter` 0))
    (`KismetSystemLibrary.Delay` (`self.DelayBeforeOnScreen`))
    (`/Engine/EditorBlueprintResources/StandardMacros.DoOnce` false
      (:`Completed`
        (`self.Display`)
        (`self.Remove`)))))

(event `Display`
  (bind _returnvalue (`|CreateWidget` "/Game/GreenOne/Widget/PopUp/WBP_DynamicPopUp.WBP_DynamicPopUp_C"))
  (bind _output_get (set `self.DynamicPopUp` _returnvalue))
  (`UserWidget.AddToViewport` _output_get 0)
  (if (`KismetSystemLibrary.DoesImplementInterface` (`self.DynamicPopUp`) "/Game/GreenOne/Blueprints/Gameplay/DynamicPopUp/BPI_DynamicPopUp.BPI_DynamicPopUp_C")
    (message `/Game/GreenOne/Blueprints/Gameplay/DynamicPopUp/BPI_DynamicPopUp.UpdatePopUp` (`self.DynamicPopUp`) (`self.PopUpText`) (`self.BackgroundColor`))))

(event `Remove`
  (`KismetSystemLibrary.Delay` (`self.TimeOnScreen`))
  (`Widget.RemoveFromParent` (`self.DynamicPopUp`)))

(fn `UpdatePopUp`
  (params (InText :type Text) (InColor :type "LinearColor Structure"))
  (return))

(fn `UserConstructionScript`)