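; BP_ZoneDetection is a trigger volume that activates arenas and spawners when the player enters.
; The first overlap of its detection box by player 0's character fires it once.
; Depending on its arena and spawner flags, it searches all BP_ArenaWall and BP_Spawner actors and activates those with matching IDs.
; The construction script displays the arena ID on a text render.
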(event `self.DetectionBox.OnComponentBeginOverlap`
  (params (OverlappedComponent :type "PrimitiveComponent Object Reference") (OtherActor :type "Actor Object Reference") (OtherComp :type "PrimitiveComponent Object Reference") (OtherBodyIndex :type Integer) (bFromSweep :type Boolean) (SweepResult :type "HitResult Structure (by ref)"))
  ;[1 1 1] Detect Player
  (if (== OtherActor (`GameplayStatics.GetPlayerCharacter` 0))
    (`/Engine/EditorBlueprintResources/StandardMacros.DoOnce` false
      (:`Completed`
        (`|ExecutionSequence`
          (:`then_0`
            ;[1 1 1] Arena
            (if (`self.IsForArena`)
              (bind _outactors (`GameplayStatics.GetAllActorsOfClass` "/Game/GreenOne/Blueprints/Gameplay/Arene/BP_ArenaWall.BP_ArenaWall_C"))
              (for _array_element _outactors
                (if (== (`/Game/GreenOne/Blueprints/Gameplay/Arene/BP_ArenaWall.ArenaId` _array_element) (`self.ZArenaId`))
                  (`/Game/GreenOne/Blueprints/Gameplay/Arene/BP_ArenaWall.ActivateArena` _array_element)))))
          (:`then_1`
            ;[1 1 1] Spawner
            (if (`self.IsForSpawner`)
              (bind _outactors_2 (`GameplayStatics.GetAllActorsOfClass` "/Game/GreenOne/Blueprints/Gameplay/Spawner/BP_Spawner.BP_Spawner_C"))
              (for _array_element_2 _outactors_2
                (if (== (`/Game/GreenOne/Blueprints/Gameplay/Spawner/BP_Spawner.SpawnerId` _array_element_2) (`self.ZSpawnerId`))
                  (`/Game/GreenOne/Blueprints/Gameplay/Spawner/BP_Spawner.SpawnerActive` _array_element_2))))))))))

(fn `UserConstructionScript`
  (`TextRenderComponent.K2_SetText` (`self.TextRender`) (`KismetTextLibrary.Conv_IntToText` (`self.ZArenaId`))))