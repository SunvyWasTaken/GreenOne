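; AIC_FlyingAI is the AI controller for flying enemies, running the flying AI behavior tree on its blackboard.
; On BeginPlay it sets up BB_FlyingAI and starts BT_FlyingAI.
; When AI perception successfully senses a GreenOneCharacter, it stores that actor as the TargetPlayer blackboard key.
; Losing sight of the target does not clear the key.
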(event `self.ReceiveBeginPlay`
  (`self.UseBlackboard` "/Game/GreenOne/Blueprints/IA/BB_FlyingAI.BB_FlyingAI")
  (`self.RunBehaviorTree` "/Game/GreenOne/Blueprints/IA/BT_FlyingAI.BT_FlyingAI"))

(event `self.AIPerception.OnTargetPerceptionUpdated`
  (params (Actor :type "Actor Object Reference") (Stimulus :type "AIStimulus Structure"))
  (if (`.bSuccessfullySensed` (break `AIStimulus` Stimulus))
    (if (`KismetMathLibrary.ClassIsChildOf` (`GameplayStatics.GetObjectClass` Actor) "/Script/GreenOne.GreenOneCharacter")
      (`BlackboardComponent.SetValueAsObject` (`AIBlueprintHelperLibrary.GetBlackboard` null) "TargetPlayer" Actor))))

(fn `UserConstructionScript`)