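; Melee AI enemy character, with a looping random patrol as its only working behavior.
; RandomPatrol sets walk speed, moves the pawn via AIMoveTo to a random reachable point within a radius of its location, and calls itself again on success.
; Nothing in this graph starts the patrol or handles a failed move, and an AIMoveTo for chasing the player is left unconnected.
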(event `RandomPatrol`
  ;[1 1 1] First method RandomPatrol
  (set `CharacterMovementComponent.MaxWalkSpeed` (`self.WalkSpeed`) (`self.CharacterMovement`))
  (`|AIMoveTo` self (`NavigationSystemV1.K2_GetRandomReachablePointInRadius` (`self.K2_GetActorLocation`) 2000.0 null null) null
    (:`OnSuccess`
      (`self.RandomPatrol`))))

(fn `UserConstructionScript`)