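; BP_FlyingAI is a flying AI actor that can also be spectated by the player.
; On BeginPlay it writes its location to its controller's Blackboard as SpawnLocation.
; FollowAI spawns a SpectatorPawn attached to the Scene component and makes the first player controller possess it.
; A looping per-frame-rate timer then keeps rotating that controller from the camera toward the AI.
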(event `self.ReceiveBeginPlay`
  (`BlackboardComponent.SetValueAsVector` (`AIBlueprintHelperLibrary.GetBlackboard` (`self.GetController`)) "SpawnLocation" (`self.K2_GetActorLocation`)))

(event `FollowAI`
  (bind _returnvalue (`|SpawnActorFromClass` "/Script/Engine.SpectatorPawn" (`KismetMathLibrary.MakeTransform` (0.0 0.0 0.0)) "Undefined" "OverrideRootScale" null null))
  (`self.K2_AttachToComponent` _returnvalue (`self.Scene`) "None" "SnapToTarget" "SnapToTarget" "KeepRelative" true)
  (`Controller.Possess` (`GameplayStatics.GetPlayerController` 0) _returnvalue)
  (`KismetSystemLibrary.K2_SetTimerDelegate` (delegate `CustomEvent`) 0.016667 true))

(event `CustomEvent`
  (`self.K2_SetActorRotation` (`GameplayStatics.GetPlayerController` 0) (`KismetMathLibrary.FindLookAtRotation` (`self.K2_GetActorLocation` (`GameplayStatics.GetPlayerCameraManager` 0)) (`self.K2_GetActorLocation`)) false))

(fn `UserConstructionScript`)