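; Player character Blueprint for GreenOne that records the last ground location, sets up the in-game HUD and clamps camera pitch.
; Walking off a ledge stores a point pulled back against the velocity by Distance.
; Other falls, such as jumps, store the actor's location, with a flag stopping the following mode change from overwriting the ledge point.
; A debug J key saves through GI_GreenOne.
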(event `self.K2_OnMovementModeChanged`
  (params (PrevMovementMode :type "EMovementMode Enum" :default "MOVE_None") (NewMovementMode :type "EMovementMode Enum" :default "MOVE_None") (PrevCustomMode :type Byte) (NewCustomMode :type Byte))
  (if (`self.Condition`)
    (if (`|EnumEquality` NewMovementMode "MOVE_Falling")
      (`self.SetLastTouchLocation` (`self.K2_GetActorLocation`)))
    (else
      (set `self.Condition` true))))

(event `self.OnWalkingOffLedge`
  (params (PreviousFloorImpactNormal :type "Vector Structure (by ref)") (PreviousFloorContactNormal :type "Vector Structure (by ref)") (PreviousLocation :type "Vector Structure (by ref)") (TimeDelta :type "Float (single-precision)"))
  (bind _output_get (set `self.NewVar` (`KismetMathLibrary.Normal` (`self.GetVelocity`))))
  (`self.SetLastTouchLocation` (+ (* _output_get (* (`self.Distance`) -1.0)) PreviousLocation))
  (set `self.Condition` false))

(event `self.ReceiveBeginPlay`
  (bind _returnvalue (`GameplayStatics.GetPlayerCameraManager` 0))
  ;[0.276 0.276 0.276] Begin Play
  (bind _asplayer_controller (cast `PlayerController` (`self.GetController`)))
  (bind _returnvalue_2 (`|CreateWidget` "/Game/GreenOne/Widget/WBP_InGame.WBP_InGame_C" _asplayer_controller))
  (`UserWidget.AddToViewport` _returnvalue_2 0)
  (`WidgetBlueprintLibrary.SetInputMode_GameOnly` _asplayer_controller)
  (set `PlayerController.bShowMouseCursor` false _asplayer_controller)
  ;;[1 1 1] Clamp Camera
  (set `PlayerCameraManager.ViewPitchMin` -35.0 _returnvalue)
  (set `PlayerCameraManager.ViewPitchMax` 35.0 _returnvalue))

(event `Key|J`
  (params (Key :type "Key Structure"))
  ;[1 1 1] DEBUG
  (:`Pressed`
    (bind _asgi_green_one (cast `GI_GreenOne` (`GameplayStatics.GetGameInstance`)))
    (`GI_GreenOne.SaveGame` _asgi_green_one)))

(fn `UserConstructionScript`)