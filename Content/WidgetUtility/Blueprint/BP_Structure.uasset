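; Procedural building Blueprint whose construction script lays rows of static mesh wall segments from corner points on each floor.
; GetWallSize measures ground and floor meshes from their bounds, feeding segment length and per-floor height offsets.
; GetWallScale rounds segment count to the nearest fit and stretches segments along their length axis to fill each span.
; The loop only builds from the last three corners and places the ground mesh on every floor.
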(fn `F_LenghtWall`
  (returns (ReturnValue :type "Float (double-precision)"))
  (bind _groundwallsize (`self.GroundWallSize`))
  (return (`KismetMathLibrary.SelectFloat` (`KismetMathLibrary.SelectFloat` (`self.MiddleWallSize`) _groundwallsize (>= (`self.CurrentFloor`) 1)) _groundwallsize (`KismetMathLibrary.NearlyEqual_FloatFloat` _groundwallsize (* (`self.MiddleWallSize`) 2.0) 0.1))))

(fn `F_WallHeight`
  (returns (ReturnValue :type "Vector Structure"))
  (bind _groundwallheight (`self.GroundWallHeight`))
  (bind _currentfloor (`self.CurrentFloor`))
  (return (`KismetMathLibrary.MakeVector` 0.0 0.0 (`KismetMathLibrary.SelectFloat` (+ (* (- _currentfloor 1) (`self.MiddleWallHeight`)) _groundwallheight) (* _currentfloor _groundwallheight) (>= (`self.CurrentFloor`) 1)))))

(fn `F_WallTransform`
  (params (Index :type Integer) (CurrentPosition :type "Vector Structure") (NextPosition :type "Vector Structure") (Scale :type "Float (double-precision)"))
  (returns (ReturnValue :type "Transform Structure"))
  (bind _scale (`local.Scale`))
  (return (`KismetMathLibrary.MakeTransform` (+ (+ (`local.CurrentPosition`) (* (* (`KismetMathLibrary.Vector_Normal2D` (- CurrentPosition NextPosition)) (`local.Index`)) (* (`self.F_LenghtWall`) (`local.Scale`)))) (`self.F_WallHeight`)) (`KismetMathLibrary.Conv_VectorToRotator` (`KismetMathLibrary.Vector_Normal2D` (- (`local.CurrentPosition`) (`local.NextPosition`)))) (`KismetMathLibrary.SelectVector` (`KismetMathLibrary.MakeVector` _scale 1.0 1.0) (`KismetMathLibrary.MakeVector` 1.0 _scale 1.0) (`self.IsMeshXSize?`)))))

(fn `GetWallScale`
  (params (V1 :type "Vector Structure") (V2 :type "Vector Structure"))
  (returns (Scale :type "Float (double-precision)") (Number :type Integer))
  (bind _returnvalue (/ (`KismetMathLibrary.Vector_Distance` V1 V2) (`self.F_LenghtWall`)))
  (bind _returnvalue_2 (mod _returnvalue 1.0))
  (bind _returnvalue_3 (>= _returnvalue_2 0.499))
  (bind _returnvalue_4 (- _returnvalue _returnvalue_2))
  (bind _returnvalue_5 (`KismetMathLibrary.FTrunc` _returnvalue_4))
  (return (`KismetMathLibrary.SelectFloat` (/ _returnvalue (+ _returnvalue_4 1.0)) (/ _returnvalue _returnvalue_4) _returnvalue_3) (`KismetMathLibrary.SelectInt` _returnvalue_5 (- _returnvalue_5 1) _returnvalue_3)))

(fn `GetWallSize`
  (if (`KismetSystemLibrary.IsValid` (`self.ListMeshGround`))
    (set `self.GroundWallSize` (`KismetMathLibrary.SelectFloat` (.x (* (`.BoxExtent` (`KismetMathLibrary.BreakBoxSphereBounds` (`StaticMesh.GetBounds` (`self.ListMeshGround`)))) 2)) (.y (* (`.BoxExtent` (`KismetMathLibrary.BreakBoxSphereBounds` (`StaticMesh.GetBounds` (`self.ListMeshGround`)))) 2)) (`self.IsMeshXSize?`)))
    (set `self.GroundWallHeight` (.z (* (`.BoxExtent` (`KismetMathLibrary.BreakBoxSphereBounds` (`StaticMesh.GetBounds` (`self.ListMeshGround`)))) 2))))
  (if (`KismetSystemLibrary.IsValid` (`self.ListMeshFloor`))
    (set `self.MiddleWallSize` (`KismetMathLibrary.SelectFloat` (.x (* (`.BoxExtent` (`KismetMathLibrary.BreakBoxSphereBounds` (`StaticMesh.GetBounds` (`self.ListMeshFloor`)))) 2)) (.y (* (`.BoxExtent` (`KismetMathLibrary.BreakBoxSphereBounds` (`StaticMesh.GetBounds` (`self.ListMeshFloor`)))) 2)) (`self.IsMeshXSize?`)))
    (set `self.MiddleWallHeight` (.z (* (`.BoxExtent` (`KismetMathLibrary.BreakBoxSphereBounds` (`StaticMesh.GetBounds` (`self.ListMeshFloor`)))) 2))))
  (return))

(fn `UserConstructionScript`
  (locals (CurrentLocation :type "Vector Structure") (NextLocation :type "Vector Structure" :default (0.0 0.0 0.0)) (PreviousLocation :type "Vector Structure" :default (0.0 0.0 0.0)) (Scale :type "Float (double-precision)" :default 0.0) (Number :type Integer :default 0))
  (bind _returnvalue (`KismetArrayLibrary.Array_Length` (`self.ListCorner`)))
  (bind _returnvalue_2 (`KismetArrayLibrary.Array_Length` (`self.ListCorner`)))
  (bind (_scale _number) (`self.GetWallScale` (`local.CurrentLocation`) (`local.NextLocation`)))
  (`self.GetWallSize`)
  (for _index (range (+ (`self.NbrFloor`) 1))
    (set `self.CurrentFloor` _index)
    (set `self.CurrentWall` 0)
    (for (_array_element _array_index) (`self.ListCorner`)
      (if (<= (- (`KismetArrayLibrary.Array_Length` (`self.ListCorner`)) 3) _array_index)
        (set `local.CurrentLocation` _array_element)
        (set `self.CurrentWall` _array_index)
        (set `local.NextLocation` (`|GetArrayItem` (`self.ListCorner`) (`KismetMathLibrary.SelectInt` (- _returnvalue_2 -1) (+ _array_index 1) (>= _array_index _returnvalue_2))))
        (set `local.PreviousLocation` (`|GetArrayItem` (`self.ListCorner`) (`KismetMathLibrary.SelectInt` (- _returnvalue -1) 0 (>= 0 _returnvalue))))
        (set `local.Scale` _scale)
        (set `local.Number` _number)
        (for _index_2 (range (+ (`local.Number`) 1))
          (bind _returnvalue_3 (`AddComponent|NODE_AddStaticMeshComponent-0` :`RelativeTransform` (`self.F_WallTransform` _index_2 (`local.CurrentLocation`) (`local.NextLocation`) (`local.Scale`))))
          (`StaticMeshComponent.SetStaticMesh` _returnvalue_3 (`self.ListMeshGround`)))))))